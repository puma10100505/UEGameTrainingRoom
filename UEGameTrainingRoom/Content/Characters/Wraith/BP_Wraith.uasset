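; BP_Wraith is the Wraith character Blueprint, which adds only an on-screen debug readout to its parent class.
; Each Tick calls the parent, then prints the current max walk speed and the IsPreparingFire state without logging.
; A Switch Has Authority colors the text green on the authority and orange on remotes, so server and client values can be compared.
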(event EventBeginPlay
  (|CallParentFunction) ; This node is disabled and will not be called.\nDrag off pins to build functionality.
)

(event Collision|EventActorBeginOverlap
  (params (OtherActor :type Actor%20Object%20Reference))
  (|CallParentFunction OtherActor) ; This node is disabled and will not be called.\nDrag off pins to build functionality.
)

(event EventTick
  (params (DeltaSeconds :type Float%20%28single-precision%29))
  (|CallParentFunction DeltaSeconds)
  (Networking|SwitchHasAuthority
    (:Authority
      (Development|PrintString (Utilities|String|ToString(Text) (Utilities|Text|FormatText "Current max move speed: {0}, Preparing Fire: {1}" (Variables|/Script/Engine.CharacterMovementComponent|GetMaxWalkSpeed (Variables|Character|GetCharacterMovement)) (Variables|Default|GetbIsPreparingFire))) true false "(R=0.020211,G=1.000000,B=0.248746,A=1.000000)" 0.0))
    (:Remote
      (Development|PrintString (Utilities|String|ToString(Text) (Utilities|Text|FormatText "Current max move speed: {0}, Preparing Fire: {1}" (Variables|/Script/Engine.CharacterMovementComponent|GetMaxWalkSpeed (Variables|Character|GetCharacterMovement)) (Variables|Default|GetbIsPreparingFire))) true false "(R=1.000000,G=0.404397,B=0.000000,A=1.000000)" 0.0))))

(fn ConstructionScript
  (|CallParentFunction))