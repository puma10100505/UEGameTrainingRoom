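; Base character Blueprint that handles shutdown after death and possession events.
; On death, an AI-controlled character with a valid brain component stops its logic, then runs ClientDeathProcess, which disables input for player controller 0 and unpossesses the character.
; Possession by a player controller calls HideHeadUpUI, but that event is empty.
; Head-up widget initialization and local-player hiding logic sit disconnected and never run.
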(event Custom|HideHeadUpUI
  (params (PlayerController :type Player%20Controller%20Object%20Reference)))

(event Custom|ClientDeathProcess
  (Input|DisableInput (Game|GetPlayerController 0))
  (Pawn|UnPossess (Pawn|GetController)))

(event EventAfterCharacterDeath
  (bind _asaicontroller_base (Utilities|Casting|CastToAIControllerBase (Pawn|GetController)))
  (if (Utilities|IsValid (Variables|/Script/AIModule.AIController|GetBrainComponent _asaicontroller_base))
    (AI|Logic|StopLogic (Variables|/Script/AIModule.AIController|GetBrainComponent _asaicontroller_base) "Characger Death")
    (CallFunction|ClientDeathProcess)))

(event EventPossessed
  (params (NewController :type Controller%20Object%20Reference))
  (bind _asplayer_controller (Utilities|Casting|CastToPlayerController NewController))
  (CallFunction|HideHeadUpUI _asplayer_controller))

(event EventBeginPlay)

(fn ConstructionScript)