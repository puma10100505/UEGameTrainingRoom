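; BP_WraithAI is an AI character Blueprint for the Wraith that relies on its parent class for its behavior.
; BeginPlay, overlap, Tick and the construction script all forward to the parent.
; Tick also serves as a debug readout, printing current Health and Armor from the health attribute set, plus the IsDead flag, on screen each frame when that set is valid.
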(event EventBeginPlay
  (|CallParentFunction))

(event Collision|EventActorBeginOverlap
  (params (OtherActor :type Actor%20Object%20Reference))
  (|CallParentFunction OtherActor))

(event EventTick
  (params (DeltaSeconds :type Float%20%28single-precision%29))
  (bind _attributesethealth (Variables|Default|GetAttributeSetHealth))
  (|CallParentFunction DeltaSeconds)
  (if (Utilities|IsValid _attributesethealth)
    (Development|PrintString (Utilities|String|ToString(Text) (Utilities|Text|FormatText "Health: {0}, Armor: {1}, IsDead: {2}" (.CurrentValue (Utilities|Struct|BreakGameplayAttributeData (Variables|/Script/UEGameTrainingRoom.AttributeSetHealth|GetHealth _attributesethealth))) (.CurrentValue (Utilities|Struct|BreakGameplayAttributeData (Variables|/Script/UEGameTrainingRoom.AttributeSetHealth|GetArmor _attributesethealth))) (Variables|Default|GetbIsDead))) true false "(R=0.000000,G=1.000000,B=0.112528,A=1.000000)" 0.0)))

(fn ConstructionScript
  (|CallParentFunction))